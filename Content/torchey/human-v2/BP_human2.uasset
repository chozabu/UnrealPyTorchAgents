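; Ragdoll humanoid agent for reinforcement learning, trained to stay upright and walk toward a randomly placed target, driven by a Python component each tick.
; Observations combine orientation, joint and body states, ground distances, decaying contacts and target angle.
; Actions set motor targets on constraints, sized by unlocked axes, while an upward head force assists balance.
; Reward scores balance, head height, progress, heading, effort and pose, ending episodes on head-height failure.
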(event `self.ReceiveBeginPlay`
  (`self.SetActorTickEnabled` false)
  (`|ExecutionSequence`
    (:`then_0`
      (`self.check_init`))
    (:`then_1`
      (`KismetSystemLibrary.Delay` 0.02)
      (`PythonComponent.CallPythonComponentMethod` (`self.Python`) "post_init" "")
      (`self.SetActorTickEnabled` true))))

(event `self.ReceiveTick`
  (params (DeltaSeconds :type "Float (single-precision)"))
  (bind _touching_ground (`self.touching_ground`))
  (if (`self.has_init`)
    (`|ExecutionSequence`
      (:`then_0`
        ;[1 1 1] check touching ground
        (bind _keys (`BlueprintMapLibrary.Map_Keys` _touching_ground))
        (for _array_element _keys
          (`BlueprintMapLibrary.Map_Add` _touching_ground _array_element (`KismetMathLibrary.SelectFloat` 0.99 0.0 (== (`BlueprintMapLibrary.Map_Find` _touching_ground _array_element) 1.0)))))
      (:`then_2`
        ;[1 1 1] draw debug info
        (`SceneComponent.SetWorldScale3D` (`self.eval_cone`) (`KismetMathLibrary.MakeVector` 0.25 0.25 (* (`self.action_eval`) 0.1)))
        (`SceneComponent.SetWorldScale3D` (`self.reward_cone`) (`KismetMathLibrary.MakeVector` 0.25 0.25 (* (`self.last_reward`) 1.0))))
      (:`then_3`
        ;[1 1 1] PythonTick
        (`PythonComponent.CallPythonComponentMethod` (`self.Python`) "pytick" ""))
      (:`then_5`
        ;[1 1 1] balance assist
        (`PrimitiveComponent.AddForce` (`self.SkeletalMesh`) (0.0 0.0 60000.0) "head" false)))
    (else
      ;[1 1 1] reinit
      (if (not (`self.has_init`))
        (`KismetSystemLibrary.Delay` 0.0)
        (`self.check_init`)))))

(event `self.ReceiveHit`
  (params (MyComp :type "PrimitiveComponent Object Reference") (Other :type "Actor Object Reference") (OtherComp :type "PrimitiveComponent Object Reference") (bSelfMoved :type Boolean) (HitLocation :type "Vector Structure") (HitNormal :type "Vector Structure") (NormalImpulse :type "Vector Structure") (Hit :type "HitResult Structure (by ref)"))
  (`BlueprintMapLibrary.Map_Add` (`self.touching_ground`) (`.ReturnValue` (`SkinnedMeshComponent.FindClosestBone_K2` (`self.SkeletalMesh`) HitLocation 0.0 true)) 1.0))

(fn `calc_reward`
  (returns (ReturnValue :type "Float (double-precision)"))
  (locals (force :type "Float (double-precision)") (dist_change :type "Float (double-precision)" :default 0.0) (lpos :type "Float (double-precision)"))
  (bind (_returnvalue_x _returnvalue_y _returnvalue_z) (`KismetMathLibrary.BreakVector` (`self.GetActorUpVector`)))
  (bind _head_ground_dist (`self.head_ground_dist`))
  (bind _returnvalue (`KismetMathLibrary.VSize` (- (`SceneComponent.GetSocketLocation` (`self.SkeletalMesh`) "Pelvis") (`SceneComponent.K2_GetComponentLocation` (`self.Target`)))))
  (`|ExecutionSequence`
    (:`then_0`
      ;[1 1 1] early fail
      (if (or (> _head_ground_dist 0.99) (<= _head_ground_dist 0.15))
        (set `self.done` true)
        (return -30.0)))
    (:`then_1`
      (`|ExecutionSequence`
        (:`then_0`
          ;[1 1 1] calc force
          (set `local.force` 0.0)
          (for _array_element (`self.phys_constraint_names`)
            (bind _returnvalue_2 (`HelperFunLib.GetSkelConstraintAngularForce` (`self.SkeletalMesh`) (`KismetStringLibrary.Conv_StringToName` _array_element)))
            (set `local.force` (+ (`local.force`) (* (`KismetMathLibrary.VSize` _returnvalue_2) 0.0001)))))
        (:`then_1`
          ;[1 1 1] neutral pos
          (set `local.lpos` 0.0)
          (for _array_element_2 (`self.joint_obs`)
            (set `local.lpos` (+ (- (`KismetMathLibrary.Abs` (- _array_element_2 0.5)) 0.1) (`local.lpos`)))))
        (:`then_2`
          ;[1 1 1] getting closer to target
          (set `local.dist_change` (- (`self.last_target_dist`) _returnvalue))
          (bind _output_get (set `self.last_target_dist` _returnvalue))
          ;[1 1 1] New Target!
          (if (< _output_get 400.0)
            (`self.reset_target_location`)))))
    (:`then_2`
      (bind _output_get_2 (set `self.last_reward` (+ (* (`local.force`) -1e-05) (* _returnvalue_z 0.2) (* (`local.dist_change`) 0.05) (* (- _head_ground_dist (`self.last_head_ground_dist`)) 100.0) (* (- 0.2 (`KismetMathLibrary.Abs` (- (`self.target_angle`) 0.5))) 0.5) (* (`local.lpos`) -0.002) (- (`self.head_ground_dist`) 0.2) 0.0)))
      (set `self.last_head_ground_dist` (`self.head_ground_dist`))
      (return _output_get_2))))

(fn `check_init`
  (bind _skeletalmesh (`self.SkeletalMesh`))
  (bind _skeletalmesh_2 (`self.SkeletalMesh`))
  (if (not (`self.has_init`))
    (`|ExecutionSequence`
      (:`then_0`
        ;[1 1 1] set init and store transform
        (set `self.has_init` true)
        (set `self.initial_transform` (`self.GetTransform`)))
      (:`then_1`
        ;[1 1 1] enable ragdoll
        (`PrimitiveComponent.SetSimulatePhysics` _skeletalmesh true)
        (`SkeletalMeshComponent.SetAllBodiesSimulatePhysics` _skeletalmesh true)
        (`PrimitiveComponent.SetCollisionEnabled` _skeletalmesh "QueryAndPhysics"))
      (:`then_2`
        ;[1 1 1] bone and constraint names
        (`KismetArrayLibrary.Array_Clear` (`self.phys_bone_names`))
        (for _array_element (`SceneComponent.GetAllSocketNames` _skeletalmesh_2)
          (if (== _array_element (`.ReturnValue` (`SkinnedMeshComponent.FindClosestBone_K2` _skeletalmesh_2 (`SceneComponent.GetSocketLocation` _skeletalmesh_2 _array_element) 0.0 true)))
            (`KismetArrayLibrary.Array_Add` (`self.phys_bone_names`) _array_element)
            (`BlueprintMapLibrary.Map_Add` (`self.touching_ground`) _array_element))))
      (:`then_3`
        ;[1 1 1] constraint names
        (bind _returnvalue (`HelperFunLib.GetConstraintNames` _skeletalmesh_2))
        (bind _output_get (set `self.phys_constraint_names` _returnvalue))
        ;[1 1 1] get locked joints
        (for _array_element_2 _output_get
          (bind _returnvalue_2 (`KismetStringLibrary.Conv_StringToName` _array_element_2))
          (bind _returnvalue_3 (`HelperFunLib.GetJointUnlocked` (`self.SkeletalMesh`) _returnvalue_2))
          (`BlueprintMapLibrary.Map_Add` (`self.joint_locks`) _returnvalue_2 _returnvalue_3)))
      (:`then_4`
        (`self.reset_target_location`))
      (:`then_5`
        (for _array_element_3 (`self.phys_constraint_names`)
          (`HelperFunLib.SetupJoint` (`self.SkeletalMesh`) (`KismetStringLibrary.Conv_StringToName` _array_element_3) 10000.0 100.0 10000.0)))
      (:`then_6`
        ;[1 1 1] enable motor
        (`SkeletalMeshComponent.SetAllMotorsAngularVelocityDrive` (`self.SkeletalMesh`) true true false)))))

(fn `extract_action`
  (params (InputPin :type "Name (by ref)") (InputPin1 :type "Array of Float (double-precision)") (InputPin2 :type Integer))
  (returns (ReturnValue :type "Rotator Structure") (ReturnValue2 :type Integer))
  (bind _joint_force (`self.joint_force`))
  (bind _x (.x (`BlueprintMapLibrary.Map_Find` (`self.joint_locks`) InputPin)))
  (bind _y (.y (`BlueprintMapLibrary.Map_Find` (`self.joint_locks`) InputPin)))
  (bind _returnvalue (+ InputPin2 (`KismetMathLibrary.Round` _x)))
  (bind _returnvalue_2 (`KismetMathLibrary.Round` (+ (+ _x _y) (.z (`BlueprintMapLibrary.Map_Find` (`self.joint_locks`) InputPin)))))
  (if (> _returnvalue_2 0)
    (return (`KismetMathLibrary.MakeRotator` (* (`|GetArrayItem` InputPin1 InputPin2) _joint_force) (* (`|GetArrayItem` InputPin1 _returnvalue) _joint_force) (* (`|GetArrayItem` InputPin1 (+ _returnvalue (`KismetMathLibrary.Round` _y))) _joint_force)) _returnvalue_2)
    (else
      (return (struct) 0))))

(fn `get_action_dim`
  (returns (ReturnValue :type Integer))
  (locals (cdim :type Integer))
  (`|ExecutionSequence`
    (:`then_0`
      (set `local.cdim` 0))
    (:`then_1`
      (`self.check_init`))
    (:`then_2`
      (bind _values (`BlueprintMapLibrary.Map_Values` (`self.joint_locks`)))
      (for _array_element _values
        (set `local.cdim` (+ (`KismetMathLibrary.Round` (+ (+ (.x _array_element) (.y _array_element)) (.z _array_element))) (`local.cdim`))))
      (return (`local.cdim`)))))

(fn `GetTargetAngleFromPos`
  (params (Target :type "Vector Structure (by ref)"))
  (returns (`Z (Yaw)` :type "Float (double-precision)"))
  (bind _returnvalue (`self.K2_GetActorLocation`))
  (`KismetSystemLibrary.DrawDebugArrow` _returnvalue (+ _returnvalue (* (`self.GetActorForwardVector`) 200.0)) 0.0 (struct :`G` 0.119515 :`B` 1.0 :`A` 1.0) 0.1 2.0)
  (return (.yaw (`KismetMathLibrary.NormalizedDeltaRotator` (`KismetMathLibrary.FindLookAtRotation` (`self.K2_GetActorLocation`) Target) (`self.K2_GetActorRotation`)))))

(fn `observe_bone`
  (params (InputPin :type "Array of Float (double-precision) (by ref)") (InputPin1 :type Name))
  (bind _skeletalmesh (`self.SkeletalMesh`))
  (bind _returnvalue (`SceneComponent.K2_GetComponentToWorld` _skeletalmesh))
  (bind (_returnvalue_x _returnvalue_y _returnvalue_z) (`KismetMathLibrary.BreakVector` (+ (* (.location (`SceneComponent.GetSocketTransform` _skeletalmesh InputPin1 "RTS_ParentBoneSpace")) 0.001) 0.5)))
  (bind (_returnvalue_x_2 _returnvalue_y_2 _returnvalue_z_2) (`KismetMathLibrary.BreakVector` (+ (* (`KismetMathLibrary.InverseTransformDirection` _returnvalue (`PrimitiveComponent.GetPhysicsAngularVelocityInRadians` _skeletalmesh InputPin1)) 0.001) 0.5)))
  (bind (_returnvalue_x_3 _returnvalue_y_3 _returnvalue_z_3) (`KismetMathLibrary.BreakVector` (+ (* (`KismetMathLibrary.MakeVector` (.roll (.rotation (`SceneComponent.GetSocketTransform` _skeletalmesh InputPin1 "RTS_ParentBoneSpace"))) (.pitch (.rotation (`SceneComponent.GetSocketTransform` _skeletalmesh InputPin1 "RTS_ParentBoneSpace"))) (.yaw (.rotation (`SceneComponent.GetSocketTransform` _skeletalmesh InputPin1 "RTS_ParentBoneSpace")))) 0.5) 0.5)))
  (bind _returnvalue_2 (`PrimitiveComponent.GetPhysicsLinearVelocity` _skeletalmesh InputPin1))
  (`KismetArrayLibrary.Array_Add` InputPin _returnvalue_x_2)
  (`KismetArrayLibrary.Array_Add` InputPin _returnvalue_y_2)
  (`KismetArrayLibrary.Array_Add` InputPin _returnvalue_z_2)
  (bind (_returnvalue_x_4 _returnvalue_y_4 _returnvalue_z_4) (`KismetMathLibrary.BreakVector` (+ (* (`KismetMathLibrary.InverseTransformDirection` _returnvalue _returnvalue_2) 0.0001) 0.5)))
  (`KismetArrayLibrary.Array_Add` InputPin _returnvalue_x_4)
  (`KismetArrayLibrary.Array_Add` InputPin _returnvalue_y_4)
  (`KismetArrayLibrary.Array_Add` InputPin _returnvalue_z_4)
  (`KismetArrayLibrary.Array_Add` InputPin _returnvalue_x)
  (`KismetArrayLibrary.Array_Add` InputPin _returnvalue_y)
  (`KismetArrayLibrary.Array_Add` InputPin _returnvalue_z)
  (`KismetArrayLibrary.Array_Add` InputPin _returnvalue_x_3)
  (`KismetArrayLibrary.Array_Add` InputPin _returnvalue_y_3)
  (`KismetArrayLibrary.Array_Add` InputPin _returnvalue_z_3))

(fn `reset_dude`
  (bind _skeletalmesh (`self.SkeletalMesh`))
  (bind _initial_transform (`self.initial_transform`))
  ;[1 1 1] disable ragdoll
  (`PrimitiveComponent.SetSimulatePhysics` _skeletalmesh false)
  (`SkeletalMeshComponent.SetAllBodiesSimulatePhysics` _skeletalmesh false)
  (`PrimitiveComponent.SetCollisionEnabled` _skeletalmesh "NoCollision")
  ;[1 1 1] reset location
  (`self.K2_SetActorTransform` _initial_transform)
  (`SceneComponent.K2_SetWorldTransform` (`self.SkeletalMesh`) _initial_transform false false)
  (set `self.has_init` false))

(fn `reset_target_location`
  (bind _returnvalue (`self.K2_GetActorLocation`))
  (bind _target (`self.Target`))
  (`SceneComponent.K2_SetWorldLocation` _target (+ (* (`KismetMathLibrary.Normal` (* (`KismetMathLibrary.RandomUnitVector`) (1.0 1.0 0.0))) 2000.0) _returnvalue (0.0 0.0 100.0)) false true)
  (set `self.last_target_dist` (`KismetMathLibrary.VSize` (- _returnvalue (`SceneComponent.K2_GetComponentLocation` _target)))))

(fn `set_action`
  (params (Array :type "Array of Float (double-precision)"))
  (locals (current_index :type Integer) (test_action_array :type "Array of Float (double-precision)"))
  (set `local.current_index` 0)
  (for _array_element (`self.phys_constraint_names`)
    (bind _returnvalue (`KismetStringLibrary.Conv_StringToName` _array_element))
    (bind (_returnvalue_2 _returnvalue2) (`self.extract_action` _returnvalue Array (`local.current_index`)))
    (`HelperFunLib.SetOrientationTarget` (`self.SkeletalMesh`) _returnvalue _returnvalue_2)
    (set `local.current_index` (+ (`local.current_index`) _returnvalue2))))

(fn `update_observation`
  (returns (observation_state :type "Array of Float (double-precision)"))
  (bind _observation_state (`self.observation_state`))
  (bind _joint_obs (`self.joint_obs`))
  (bind _observation_state_2 (`self.observation_state`))
  (bind _returnvalue (`SceneComponent.GetSocketLocation` (`self.SkeletalMesh`) "Pelvis"))
  (bind _returnvalue_2 (`SceneComponent.GetSocketLocation` (`self.SkeletalMesh`) "Head"))
  (bind _rotation (.rotation (`SceneComponent.K2_GetComponentToWorld` (`self.Arrow`))))
  (bind (_x _y _z) (`KismetMathLibrary.BreakRotIntoAxes` _rotation))
  ;[1 1 1] ActorMatch Ragdoll
  (`self.K2_SetActorLocation` (.location (`SceneComponent.K2_GetComponentToWorld` (`self.Arrow`))))
  (`self.K2_SetActorRotation` _rotation)
  ;[1 1 1] clear obs
  (`KismetArrayLibrary.Array_Clear` (`self.observation_state`))
  (`KismetArrayLibrary.Array_Clear` (`self.joint_obs`))
  ;[1 1 1] observe balance
  (`KismetArrayLibrary.Array_Add` _observation_state_2 (.x _x))
  (`KismetArrayLibrary.Array_Add` _observation_state_2 (.y _x))
  (`KismetArrayLibrary.Array_Add` _observation_state_2 (.z _x))
  (`KismetArrayLibrary.Array_Add` _observation_state_2 (.x _y))
  (`KismetArrayLibrary.Array_Add` _observation_state_2 (.y _y))
  (`KismetArrayLibrary.Array_Add` _observation_state_2 (.z _y))
  (`KismetArrayLibrary.Array_Add` _observation_state_2 (.x _z))
  (`KismetArrayLibrary.Array_Add` _observation_state_2 (.y _z))
  (`KismetArrayLibrary.Array_Add` _observation_state_2 (.z _z))
  ;[1 1 1] observe joints
  (for _array_element (`self.phys_constraint_names`)
    (bind _returnvalue_3 (`HelperFunLib.GetOrientation` (`self.SkeletalMesh`) (`KismetStringLibrary.Conv_StringToName` _array_element)))
    (bind _x_2 (.x (+ (/ _returnvalue_3 (* (`KismetMathLibrary.GetPI`) 2.0)) 0.5)))
    (bind _y_2 (.y (+ (/ _returnvalue_3 (* (`KismetMathLibrary.GetPI`) 2.0)) 0.5)))
    (bind _z_2 (.z (+ (/ _returnvalue_3 (* (`KismetMathLibrary.GetPI`) 2.0)) 0.5)))
    (`KismetArrayLibrary.Array_Add` _observation_state _x_2)
    (`KismetArrayLibrary.Array_Add` _observation_state _y_2)
    (`KismetArrayLibrary.Array_Add` _observation_state _z_2)
    (`KismetArrayLibrary.Array_Add` _joint_obs _x_2)
    (`KismetArrayLibrary.Array_Add` _joint_obs _y_2)
    (`KismetArrayLibrary.Array_Add` _joint_obs _z_2))
  ;[1 1 1] observe bodys
  (for _array_element_2 (`self.phys_bone_names`)
    (`self.observe_bone` (`self.observation_state`) _array_element_2))
  ;[1 1 1] dist to ground
  (bind (_outhit _returnvalue_4) (`KismetSystemLibrary.LineTraceSingle` :`Start` _returnvalue :`End` (- _returnvalue (0.0 0.0 500.0)) :`TraceChannel` "TraceTypeQuery1" :`DrawDebugType` "ForOneFrame"))
  (if _returnvalue_4
    (bind _output_get (set `self.ground_dist` (/ (`.Distance` (`GameplayStatics.BreakHitResult` _outhit)) 500.0)))
    (`KismetArrayLibrary.Array_Add` (`self.observation_state`) _output_get)
    (else
      (bind _output_get_2 (set `self.ground_dist` 1.0))
      (`KismetArrayLibrary.Array_Add` (`self.observation_state`) _output_get_2)))
  ;[1 1 1] dist to ground
  (bind (_outhit_2 _returnvalue_5) (`KismetSystemLibrary.LineTraceSingle` :`Start` _returnvalue_2 :`End` (- _returnvalue_2 (0.0 0.0 500.0)) :`TraceChannel` "TraceTypeQuery1" :`DrawDebugType` "ForOneFrame"))
  (if _returnvalue_5
    (bind _output_get_3 (set `self.head_ground_dist` (/ (`.Distance` (`GameplayStatics.BreakHitResult` _outhit_2)) 500.0)))
    (`KismetArrayLibrary.Array_Add` (`self.observation_state`) _output_get_3)
    (else
      (bind _output_get_4 (set `self.head_ground_dist` 1.0))
      (`KismetArrayLibrary.Array_Add` (`self.observation_state`) _output_get_4)))
  ;[1 1 1] touch sensiors
  (bind _values (`BlueprintMapLibrary.Map_Values` (`self.touching_ground`)))
  (`KismetArrayLibrary.Array_Append` (`self.observation_state`) _values)
  ;[1 1 1] target angle
  (bind _z__yaw_ (`self.GetTargetAngleFromPos` (`SceneComponent.K2_GetComponentLocation` (`self.Target`))))
  (bind _output_get_5 (set `self.target_angle` (+ (/ _z__yaw_ 360.0) 0.5)))
  (`KismetArrayLibrary.Array_Add` (`self.observation_state`) _output_get_5)
  (`KismetSystemLibrary.DrawDebugLine` (`self.K2_GetActorLocation`) (`SceneComponent.K2_GetComponentLocation` (`self.Target`)) (struct :`G` 1.0 :`B` 0.069329 :`A` 1.0) 0.1 2.0)
  (return (`self.observation_state`)))

(fn `UserConstructionScript`)